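; Avatar_BP is an RPG avatar Blueprint that passes an attack target from its BattleAIController to the AI blackboard.
; Its Tick logic writes any set controller target to the TargetToAttack key when a blackboard is valid, then clears the controller's target.
; BeginPlay disables actor Tick, and nothing in this Blueprint turns it back on.
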(event EventBeginPlay
  (Actor|Tick|SetActorTickEnabled false))

(event EventTick
  (params (DeltaSeconds :type Float%20%28single-precision%29))
  (bind _returnvalue (Pawn|GetController))
  (bind _returnvalue_2 (Pawn|GetControlledPawn _returnvalue))
  (bind _asbattle_aicontroller (Utilities|Casting|CastToBattleAIController _returnvalue))
  (bind _returnvalue_3 (Class|BattleAIController|GetTarget _asbattle_aicontroller))
  (bind _returnvalue_4 (AI|GetBlackboard _returnvalue_2))
  (if (not (== _returnvalue_3 0))
    (Utilities|IsValid _returnvalue_4
      (:Is%20Valid
        (AI|Components|Blackboard|SetValueasObject _returnvalue_4 (Utilities|Name|MakeLiteralName "TargetToAttack") _returnvalue_3)
        (Class|BattleAIController|SetTarget _asbattle_aicontroller)))))

(fn ConstructionScript)