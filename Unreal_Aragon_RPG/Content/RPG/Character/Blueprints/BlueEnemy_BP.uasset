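; Enemy character Blueprint for the blue enemy, linking its battle AI controller to the Blackboard and its health bar widget.
; After a one-second delay on BeginPlay it writes its Player reference to the Blackboard and sets itself as the health bar's owner.
; Tick checks the controller's target, copies it to the TargetToAttack key, then calls SetTarget with no argument, so targets act as one-shot handoffs.
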(event EventBeginPlay
  (bind _returnvalue (Pawn|GetController))
  (bind _returnvalue_2 (Pawn|GetControlledPawn _returnvalue))
  (bind _returnvalue_3 (AI|GetBlackboard _returnvalue_2))
  ;[1 1 1] Set player to blackboard
  (Utilities|FlowControl|Delay 1.0)
  (Utilities|IsValid _returnvalue_3
    (:Is%20Valid
      (bind _asenemy (Utilities|Casting|CastToEnemy _returnvalue_2))
      (AI|Components|Blackboard|SetValueasObject _returnvalue_3 (Utilities|Name|MakeLiteralName "Player") (Variables|/Script/Unreal_Aragon_RPG.Enemy|GetPlayer _asenemy))
      (CallFunction|BindHealthbartoOwner))))

(event Collision|EventActorBeginOverlap
  (params (OtherActor :type Actor%20Object%20Reference)))

(event EventTick
  (params (DeltaSeconds :type Float%20%28single-precision%29))
  (bind _returnvalue (Pawn|GetController))
  (bind _returnvalue_2 (Pawn|GetControlledPawn _returnvalue))
  (bind _asbattle_aicontroller (Utilities|Casting|CastToBattleAIController _returnvalue))
  (bind _returnvalue_3 (Class|BattleAIController|GetTarget _asbattle_aicontroller))
  (bind _returnvalue_4 (AI|GetBlackboard _returnvalue_2))
  (if (not (== _returnvalue_3 0))
    (Utilities|IsValid _returnvalue_4
      (:Is%20Valid
        (AI|Components|Blackboard|SetValueasObject _returnvalue_4 (Utilities|Name|MakeLiteralName "TargetToAttack") _returnvalue_3)
        (Class|BattleAIController|SetTarget _asbattle_aicontroller)))))

(fn ConstructionScript)

(fn BindHealthbartoOwner
  (bind _asenemy_health_bar_bp (Utilities|Casting|CastToEnemyHealthBar_BP (UserInterface|GetUserWidgetObject (Variables|Default|GetHealthbar))))
  (Variables|/Game/RPG/UI/EnemyHealthBar_BP.EnemyHealthBar_BP_C|SetOwner _asenemy_health_bar_bp self))